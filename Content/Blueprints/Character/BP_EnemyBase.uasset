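; BP_EnemyBase is the base enemy Blueprint, handling visual spawn, death-dissolve and attack-facing behavior.
; On BeginPlay a timeline scales the mesh in.
; Body and weapon dissolve events drive a Dissolve scalar on passed-in dynamic materials through timelines, with the body one also hiding the health bar.
; UpdateFacingTarget feeds a location to Motion Warping's FacingTarget warp target.
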(event `CombatInterface.UpdateFacingTarget`
  (params (Target :type "Vector Structure"))
  (`MotionWarpingComponent.AddOrUpdateWarpTargetFromLocation` (`self.MotionWarping`) "FacingTarget" Target))

(event `self.StartDissolveTimeline`
  (params (DynamicMaterialInstance :type "MaterialInstanceDynamic Object Reference"))
  (bind (_direction _dissolvetrack) (`Timeline|DissolveTimeline`)
    (:`Update`
      (`MaterialInstanceDynamic.SetScalarParameterValue` DynamicMaterialInstance "Dissolve" _dissolvetrack)
      (`SceneComponent.SetVisibility` (`self.HealthBar`) false false))))

(event `self.StartWeaponDissolveTimeline`
  (params (DynamicMaterialInstance :type "MaterialInstanceDynamic Object Reference"))
  (bind (_direction _newtrack_0) (`Timeline|WeaponDissolveTimeline`)
    (:`Update`
      (`MaterialInstanceDynamic.SetScalarParameterValue` DynamicMaterialInstance "Dissolve" _newtrack_0))))

(event `self.ReceiveBeginPlay`
  (bind (_direction _scaletrack) (`Timeline|SpawnTimeline`)
    (:`Update`
      (`SceneComponent.SetRelativeScale3D` (`self.Mesh`) (`KismetMathLibrary.MakeVector` _scaletrack _scaletrack _scaletrack)))))

(fn `UserConstructionScript`)